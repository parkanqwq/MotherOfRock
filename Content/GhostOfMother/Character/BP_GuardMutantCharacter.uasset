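; Guard mutant enemy that fires a GAS shooting ability while the player soldier is in its overlap range.
; BeginPlay grants GA_ShootMonster, and overlap starts a delay loop that simulates input press and release until the player leaves.
; Tick polls IsDeath through a Delay, then halts movement, plays a scream and destroys the actor after another delay.
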(event `self.ReceiveBeginPlay`
  (`parent.ReceiveBeginPlay`)
  (`AbilitySystemComponent.K2_GiveAbility` (`self.AbilitySystem`) "/Game/GhostOfMother/Core/GameSystem/GameplayAbilities/ShootMonster/GA_ShootMonster.GA_ShootMonster_C" 1 1))

(event `self.ReceiveActorBeginOverlap`
  (params (OtherActor :type "Actor Object Reference"))
  (bind _abilitysystem (`self.AbilitySystem`))
  (cast `/Game/GhostOfMother/Character/BP_PlayerSoldierCharacter` OtherActor)
  (set `self.IsAttack` true)
  (`KismetSystemLibrary.Delay` 1.5 :!label _label)
  (`AbilitySystemComponent.PressInputID` _abilitysystem 1)
  (`AbilitySystemComponent.ReleaseInputID` _abilitysystem 1)
  (if (`self.IsAttack`)
    (`KismetSystemLibrary.Delay` 1.5)
    (goto _label)))

(event `self.ReceiveActorEndOverlap`
  (params (OtherActor :type "Actor Object Reference"))
  (cast `/Game/GhostOfMother/Character/BP_PlayerSoldierCharacter` OtherActor)
  (set `self.IsAttack` false))

(event `self.ReceiveTick`
  (params (DeltaSeconds :type "Float (single-precision)"))
  (`KismetSystemLibrary.Delay` 0.5)
  (if (`self.IsDeath`)
    (set `CharacterMovementComponent.MaxWalkSpeed` 0.0 (`self.CharacterMovement`))
    (`GameplayStatics.PlaySoundAtLocation` "/Game/GhostOfMother/Core/Sounds/female-scream-reverse-echo-effect.female-scream-reverse-echo-effect" (0.0 0.0 0.0) (struct) 1.0 1.0 0.0 "/Game/GhostOfMother/Core/Sounds/ZA_FootStep.ZA_FootStep" null null null)
    (`KismetSystemLibrary.Delay` 3.0)
    (`self.K2_DestroyActor`)))

(fn `UserConstructionScript`
  (`parent.UserConstructionScript`))