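; Player soldier character that creates its HUD widget, controls run speed and shoots an AK47 through the Gameplay Ability System.
; Enhanced Input switches between run and walk speed, keeping walk speed while moving back, and presses or releases the granted GA_ShootPlayer ability.
; SetProgressHp updates the HUD health bar.
; Tick polls health behind a Delay; at zero it removes the rifle, ragdolls with physical animation, then destroys the actor.
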(event `self.ReceiveBeginPlay`
  (`parent.ReceiveBeginPlay`)
  (bind _returnvalue (`|CreateWidget` "/Game/GhostOfMother/Core/UI/WB_UIPlayerGameSoldier.WB_UIPlayerGameSoldier_C"))
  (`UserWidget.AddToViewport` _returnvalue 0)
  (set `self.Widget` _returnvalue)
  (`AbilitySystemComponent.K2_GiveAbility` (`self.AbilitySystem`) "/Game/GhostOfMother/Core/GameSystem/GameplayAbilities/ShootPlayer/GA_ShootPlayer.GA_ShootPlayer_C" 1 1))

(event `self.ReceiveTick`
  (params (DeltaSeconds :type "Float (single-precision)"))
  (`KismetSystemLibrary.Delay` 1.0)
  (bind _gethealth (`/Game/GhostOfMother/Character/Attributs/AC_Health.GetHealth` (`self.AC_Health`)))
  (if (<= _gethealth 0.0)
    (`self.PlayerDiead`)
    (`KismetSystemLibrary.Delay` 2.0)
    (`self.K2_DestroyActor`)))

(event `EnhancedInput|/Game/GhostOfMother/Input/Actions/IA_Run`
  (params (ActionValue :type Boolean) (ElapsedSeconds :type "Float (double-precision)") (TriggeredSeconds :type "Float (double-precision)") (InputAction :type "InputAction Object Reference" :default "/Game/GhostOfMother/Input/Actions/IA_Run.IA_Run"))
  (bind _charactermovement (`self.CharacterMovement`))
  ;[1 1 1] Бежать или идти
  (:`Started`
    (set `self.IsRun` true)
    (if (and (`self.IsRun`) (not (`self.IsWalk`)))
      (set `CharacterMovementComponent.MaxWalkSpeed` 500.0 _charactermovement)
      (else
        (set `CharacterMovementComponent.MaxWalkSpeed` 250.0 _charactermovement :!label _label))))
  (:`Completed`
    (goto _label)))

(event `EnhancedInput|/Game/GhostOfMother/Input/Actions/IA_Back`
  (params (ActionValue :type Boolean) (ElapsedSeconds :type "Float (double-precision)") (TriggeredSeconds :type "Float (double-precision)") (InputAction :type "InputAction Object Reference" :default "/Game/GhostOfMother/Input/Actions/IA_Back.IA_Back"))
  ;[1 1 1] Бежать или идти
  (:`Started`
    (set `self.IsRun` false)
    (set `self.IsWalk` true)
    (goto _label))
  (:`Completed`
    (set `self.IsWalk` false)))

(event `EnhancedInput|/Game/GhostOfMother/Input/Actions/IA_ShootAK47`
  (params (ActionValue :type Boolean) (ElapsedSeconds :type "Float (double-precision)") (TriggeredSeconds :type "Float (double-precision)") (InputAction :type "InputAction Object Reference" :default "/Game/GhostOfMother/Input/Actions/IA_ShootAK47.IA_ShootAK47"))
  (bind _abilitysystem (`self.AbilitySystem`))
  ;[1 1 1] Стрельба
  (:`Started`
    (`AbilitySystemComponent.PressInputID` _abilitysystem 1))
  (:`Completed`
    (`AbilitySystemComponent.ReleaseInputID` _abilitysystem 1)))

(fn `PlayerDiead`
  (`|ExecutionSequence`
    (:`then_0`
      (bind _ak47nosubdiv (`self.AK47NoSubdiv`)
        (:`then`
          (`ActorComponent.K2_DestroyComponent` _ak47nosubdiv))
        (:`else`)))
    (:`then_1`
      (`PhysicalAnimationComponent.SetSkeletalMeshComponent` (`self.PhysicalAnimation`) (`self.Mesh`))
      (`PhysicalAnimationComponent.ApplyPhysicalAnimationSettingsBelow` (`self.PhysicalAnimation`) (`self.BodyHips`) (make `PhysicalAnimationData` true 50.0 5.0 50.0 5.0) true)
      (`SkeletalMeshComponent.SetAllBodiesBelowSimulatePhysics` (`self.Mesh`) (`self.BodyHips`) true true)
      (`PrimitiveComponent.SetCollisionProfileName` (`self.Mesh`) "Ragdoll" true)
      (`CharacterMovementComponent.DisableMovement` (`self.CharacterMovement`)))))

(fn `SetProgressHp`
  (params (InPercent :type "Float (single-precision)"))
  (`ProgressBar.SetPercent` (`/Game/GhostOfMother/Core/UI/WB_UIPlayerGameSoldier.ProgressBar_HP` (`self.Widget`)) (/ InPercent 100.0)))

(fn `UserConstructionScript`
  (`parent.UserConstructionScript`))