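; Behavior Tree service for the mutant guard that feeds the player's position to its AI while the player is within a set distance band.
; Each tick it measures the distance from the controlled pawn to player pawn 0.
; Inside the configurable min-max range it writes the player's location to a vector blackboard key.
; When the player is out of range or invalid, it clears that key.
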(event `self.ReceiveTickAI`
  (params (OwnerController :type "AIController Object Reference") (ControlledPawn :type "Pawn Object Reference") (DeltaSeconds :type "Float (single-precision)"))
  (bind _returnvalue (`GameplayStatics.GetPlayerPawn` 0))
  (bind _key (`self.Key`))
  (bind _returnvalue_2 (`Actor.K2_GetActorLocation` _returnvalue))
  (`/Engine/EditorBlueprintResources/StandardMacros.IsValid` _returnvalue
    (:`Is Valid`
      (if (`KismetMathLibrary.InRange_FloatFloat` (`KismetMathLibrary.Vector_Distance` (`Actor.K2_GetActorLocation` ControlledPawn) _returnvalue_2) (`self.MinDistanc`) (`self.MaxDistanc`))
        (`BTFunctionLibrary.SetBlackboardValueAsVector` _key _returnvalue_2)
        (else
          (`BTFunctionLibrary.ClearBlackboardValue` _key :!label _label))))
    (:`Is Not Valid`
      (goto _label))))