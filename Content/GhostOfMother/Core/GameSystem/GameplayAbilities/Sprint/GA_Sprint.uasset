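; Gameplay ability that makes the player soldier sprint while the input is held.
; After committing, it loops on a 0.1-second delay, re-committing the cost each tick, setting IsRun and raising walk speed unless IsWalk is set.
; Walking drops the speed and stops the loop, while input release or a failed cost commit also ends the ability.
; IsRun is never cleared here.
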(event `self.K2_ActivateAbility`
  (bind _bp_player_soldier_character (`self.BP Player Soldier Character`))
  (bind _charactermovement (`Character.CharacterMovement` _bp_player_soldier_character))
  (bind _asbp_player_soldier_character (cast `/Game/GhostOfMother/Character/BP_PlayerSoldierCharacter` (`self.GetAvatarActorFromActorInfo`))
    (:`then`
      (set `self.BP Player Soldier Character` _asbp_player_soldier_character)
      (`self.K2_CommitAbility`)
      (if true
        (`AbilityTask_WaitInputRelease.WaitInputRelease` false
          (:`then`
            (`AbilityTask_WaitDelay.WaitDelay` 0.1 :!label _label
              (:`OnFinish`
                (bind _returnvalue (`self.K2_CommitAbilityCost` false))
                (if _returnvalue
                  (set `/Game/GhostOfMother/Character/BP_PlayerSoldierCharacter.IsRun` true _bp_player_soldier_character)
                  (if (and (`/Game/GhostOfMother/Character/BP_PlayerSoldierCharacter.IsRun` _bp_player_soldier_character) (not (`/Game/GhostOfMother/Character/BP_PlayerSoldierCharacter.IsWalk` _bp_player_soldier_character)))
                    (set `CharacterMovementComponent.MaxWalkSpeed` 500.0 _charactermovement)
                    (goto _label)
                    (else
                      (set `CharacterMovementComponent.MaxWalkSpeed` 250.0 _charactermovement)))
                  (else
                    (set `CharacterMovementComponent.MaxWalkSpeed` 250.0 (`Character.CharacterMovement` (`self.BP Player Soldier Character`)) :!label _label_2)
                    (`self.K2_EndAbility`))))))
          (:`OnRelease`
            (goto _label_2)))
        (else
          (`self.K2_CancelAbility`))))
    (:`CastFailed`
      (`self.K2_CancelAbility`))))