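; GA_ShootMonster is a Gameplay Ability, named as a monster's shot, that deals damage directly to the player soldier.
; On activation it finds BP_PlayerSoldierCharacter by class and commits, with no trace or projectile involved.
; A successful commit subtracts Damage from the ACHealth component, updates the HP progress display and ends the ability, then wires back to the start.
; A failed commit cancels the ability.
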(event `self.K2_ActivateAbility`
  (bind _returnvalue (`GameplayStatics.GetActorOfClass` "/Game/GhostOfMother/Character/BP_PlayerSoldierCharacter.BP_PlayerSoldierCharacter_C" :!label _label))
  (bind _returnvalue_2 (`self.K2_CommitAbility`))
  (if _returnvalue_2
    (bind _ac_health (`/Game/GhostOfMother/Character/BP_BaseCharacter.AC_Health` _returnvalue))
    (bind _gethealth (`/Game/GhostOfMother/Character/Attributs/AC_Health.GetHealth` _ac_health))
    (bind _returnvalue_3 (- _gethealth (`self.Damage`)))
    (`/Game/GhostOfMother/Character/Attributs/AC_Health.SetHealth` _ac_health _returnvalue_3)
    (`/Game/GhostOfMother/Character/BP_PlayerSoldierCharacter.SetProgressHp` _returnvalue _returnvalue_3)
    (`self.K2_EndAbility`)
    (goto _label)
    (else
      (`self.K2_CancelAbility`))))

(event `self.K2_OnEndAbility`
  (params (bWasCancelled :type Boolean)))