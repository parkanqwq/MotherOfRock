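; Gameplay ability for the player soldier's shot, covering state, feedback and effect, with no trace or projectile in this graph.
; Activation sets IsShoot, slows walking, waits briefly, then plays explosion particles and sound at the AK47 arrow.
; It applies GE_ShootPlayer and immediately ends, which clears IsShoot and removes that effect unless cancelled.
; Walk speed is not restored here, and a failed avatar check cancels the ability.
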(event `self.K2_ActivateAbility`
  (bind _returnvalue (`self.GetAvatarActorFromActorInfo`))
  (bind _returnvalue_2 (`SceneComponent.GetSocketLocation` (`self.Arrow AK47`) "None"))
  (`/Engine/EditorBlueprintResources/StandardMacros.IsValid` _returnvalue
    (:`Is Valid`
      (set `self.ActorAbilities` _returnvalue)
      (bind _asbp_player_soldier_character (cast `/Game/GhostOfMother/Character/BP_PlayerSoldierCharacter` _returnvalue)
        (:`then`
          (set `self.Character Movement` (`Character.CharacterMovement` _asbp_player_soldier_character))
          (set `self.Arrow AK47` (`/Game/GhostOfMother/Character/BP_PlayerSoldierCharacter.ArrowAK47` _asbp_player_soldier_character))
          (set `self.Follow Camera` (`/Game/GhostOfMother/Character/BP_BaseCharacter.FollowCamera` _asbp_player_soldier_character))
          (set `/Game/GhostOfMother/Character/BP_PlayerSoldierCharacter.IsShoot` true _asbp_player_soldier_character)
          (set `CharacterMovementComponent.MaxWalkSpeed` 250.0 (`self.Character Movement`))
          (`KismetSystemLibrary.Delay` 0.2)
          (`GameplayStatics.SpawnEmitterAtLocation` "/Game/StarterContent/Particles/P_Explosion.P_Explosion" _returnvalue_2 (struct) (0.01 0.01 0.01))
          (`GameplayStatics.SpawnSoundAtLocation` "/Game/StarterContent/Audio/Explosion01.Explosion01" _returnvalue_2 (struct) 1.0 1.0 0.0 "/Game/GhostOfMother/Core/Sounds/ZA_FootStep.ZA_FootStep" null)
          (bind _returnvalue_3 (`self.BP_ApplyGameplayEffectToOwner` "/Game/GhostOfMother/Core/GameSystem/GameplayAbilities/ShootPlayer/GE_ShootPlayer.GE_ShootPlayer_C"))
          (set `self.AplyedEffect` _returnvalue_3)
          (`self.K2_EndAbility`))
        (:`CastFailed`
          (`self.K2_CancelAbility`))))
    (:`Is Not Valid`
      (`self.K2_CancelAbility`))))

(event `self.K2_OnEndAbility`
  (params (bWasCancelled :type Boolean))
  (set `/Game/GhostOfMother/Character/BP_PlayerSoldierCharacter.IsShoot` false (stale `self.K2_ActivateAbility` _asbp_player_soldier_character))
  (if (not bWasCancelled)
    (`self.BP_RemoveGameplayEffectFromOwnerWithHandle` (`self.AplyedEffect`))))